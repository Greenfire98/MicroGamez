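; A moving shooting-gallery style target for a microgame that travels back and forth until hits destroy it.
; Tick offsets the actor along its normalized Direction by Speed each frame, without sweep or delta-time scaling.
; A looping timer reverses Direction every MovementDuration seconds.
; Each hit lowers HP and plays a sound; at zero it spawns an explosion effect and sound, then destroys itself.
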(event Custom|CustomEvent
  ;[0 0.7522 1] Flip Direction
  (Variables|Default|SetDirection (* (Variables|Default|GetDirection) -1.0)))

(event EventBeginPlay
  ;[0 0.7522 1] Flip Direction
  (Utilities|Time|SetTimerbyEvent (delegate Custom|CustomEvent) (Variables|Default|GetMovement_Duration) true))

(event EventTick
  (params (DeltaSeconds :type Float%20%28single-precision%29))
  ;[0 1 0.1086] Moving Target
  (Transformation|AddActorWorldOffset (* (Math|Vector|Normalize (Variables|Default|GetDirection)) (Variables|Default|GetSpeed))))

(event Collision|EventHit
  (params (MyComp :type Primitive%20Component%20Object%20Reference) (Other :type Actor%20Object%20Reference) (OtherComp :type Primitive%20Component%20Object%20Reference) (bSelfMoved :type Boolean) (HitLocation :type Vector :default "0, 0, 0") (HitNormal :type Vector :default "0, 0, 0") (NormalImpulse :type Vector :default "0, 0, 0") (Hit :type Hit%20Result%20Structure%20%28by%20ref%29))
  ;[1 0.09896 0.09896] Destroying Target
  (Variables|Default|SetHP (- (Variables|Default|GetHP) 1))
  (if (<= (Variables|Default|GetHP) 0)
    (Effects|SpawnEmitteratLocation "/Game/StarterContent/Particles/P_Explosion.P_Explosion" HitLocation)
    (Audio|PlaySoundatLocation "/Game/StarterContent/Audio/Explosion01.Explosion01" HitLocation "0, 0, 0" 1.0 1.0 0.0 0 0 0 0)
    (Actor|DestroyActor)
    (else
      (Audio|PlaySoundatLocation "/Game/StarterContent/Audio/Explosion_Cue.Explosion_Cue" HitLocation "0, 0, 0" 1.0 1.0 0.0 0 0 0 0))))

(fn ConstructionScript
  (|CallParentFunction))